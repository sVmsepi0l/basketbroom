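; Dungeon entrance or exit actor, configured by a data table row, that registers a transient entrance beacon and loads the dungeon level.
; Construction derives the lock type and spawns the dungeon type's geometry as a child actor.
; Mission, stat, database, time-of-day or switch locks gate interaction and looping audio, rechecked on overlap, switch or Hermes events.
; Level loading can disable companions, adds exit start-tag options and sets the respawn reason.
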(event OnComponentBeginOverlap(Sphere)
  (params (OverlappedComponent :type Primitive%20Component%20Object%20Reference) (OtherActor :type Actor%20Object%20Reference) (OtherComp :type Primitive%20Component%20Object%20Reference) (OtherBodyIndex :type Integer) (bFromSweep :type Boolean) (SweepResult :type Hit%20Result%20Structure%20%28by%20ref%29))
  (bind _interactactor (Variables|Runtime|GetInteractActor))
  (bind _cognitionstimulisource (Variables|/Game/Gameplay/Dungeons/BluePrints/BP_DungeonInteract.BP_DungeonInteract_C|GetCognitionStimuliSource _interactactor))
  ;[1 1 1] Check to see if the interact should be on. I don't like this, but it works for now.
  ;[1 1 1] Lock, Stat, Mission checks
  (switch Utilities|FlowControl|Switch|SwitchonE_DungeonEntranceLockTypes (Variables|Runtime|GetLockType)
    (:NewEnumerator5
      ;[1 1 1] Register for interact or not based on stat,lock,or mission check
      (Variables|Runtime|SetEnableAudio true :!label _label)
      (Class|AIPerceptionStimuliSourceComponent|RegisterforSense _cognitionstimulisource "/Script/Phoenix.AISense_CogGroup_Interact")
      (CallFunction|AudioCheck))
    (:NewEnumerator0
      (bind _missioncheckpassed (CallFunction|MissionStateCheck))
      (if _missioncheckpassed
        (goto _label)
        (else
          (Variables|Runtime|SetEnableAudio false :!label _label_2)
          (Class|AIPerceptionStimuliSourceComponent|UnregisterfromSense _cognitionstimulisource "/Script/Phoenix.AISense_CogGroup_Interact"))))
    (:NewEnumerator1
      (bind _load (CallFunction|StatCheck))
      (if _load
        (goto _label)
        (else
          (goto _label_2))))
    (:NewEnumerator2
      (bind _lockpassed (CallFunction|LockCheck))
      (if _lockpassed
        (goto _label)
        (else
          (goto _label_2))))
    (:NewEnumerator3
      (bind _checkpassed (CallFunction|DayNightCheck))
      (if _checkpassed
        (goto _label)
        (else
          (goto _label_2))))
    (:NewEnumerator4
      (if (Variables|Runtime|GetSwitchActive)
        (goto _label)
        (else
          (goto _label_2))))))

(event Custom|AudioCheck
  ;[1 1 1] Audio
  (if (Variables|Runtime|GetEnableAudio)
    (bind _returnvalue (Class|AkGameplayStatics|GetAkComponent 0 "None" (+ (Transformation|GetActorLocation self) "-1230.000000,0.000000,252.000000") "KeepRelativeOffset"))
    (Utilities|IsValid _returnvalue
      (:Is%20Valid
        (Class|AkGameObject|PostAkEvent _returnvalue "/Game/WWise/Events/InteractiveObjects/BP_DungeonLOCs/BP_DungeonLOCs_Gate_Energy_Loop.BP_DungeonLOCs_Gate_Energy_Loop")
        (Class|AkComponent|SetStopwhenOwnerDestroyed _returnvalue true)))))

(event Custom|DungeonLocsInteractUpdate
  (params (Caller :type Object%20Object%20Reference))
  (CallFunction|UpdateInteractCheck))

(event Custom|RegisterDungeon
  (bind _entrancedata (Variables|Runtime|GetEntranceData))
  (bind _entrancedata_2 (Variables|Runtime|GetEntranceData))
  (bind _dungeonlocation (Variables|Default|GetDungeonLocation))
  (bind _dungeonname (Variables|Default|GetDungeonName))
  (bind _dungeonname_2 (Variables|Default|GetDungeonName))
  (bind _isexit (Utilities|Struct|BreakSTR_TransientDungeonListData _entrancedata))
  (bind _isexit_2 (Utilities|Struct|BreakSTR_TransientDungeonListData _entrancedata_2))
  (bind _returnvalue (Transformation|GetWorldLocation _dungeonlocation))
  (bind _returnvalue_2 (Utilities|String|ToString(Name) (.dungeonname _dungeonname_2)))
  (bind _returnvalue_3 (Transformation|GetWorldRotation _dungeonlocation))
  (bind _returnvalue_4 (Utilities|String|Replace _returnvalue_2 "Gobmine" "GobMine"))
  (bind _yaw (Math|Rotator|BreakRotator _returnvalue_3))
  (bind _returnvalue_5 (select _isexit_2 1 0))
  (bind _returnvalue_6 (Utilities|String|Append _returnvalue_4 "_EXIT"))
  (bind _returnvalue_7 (Utilities|String|SelectString _returnvalue_6 _returnvalue_4 _isexit))
  ;[1 1 1] Register Dungeon
  (bind _returnvalue_8 (Utilities|GetDataTableRow (.datatable _dungeonname) (.dungeonname _dungeonname))
    (:then
      (if (Utilities|IsValidSoftObjectReference (Class|PhoenixBPLibrary|CasttoWorldSoftObjectReference (.DungeonLevel (Utilities|Struct|BreakSTR_TransientDungeonListData _returnvalue_8))))
        ;[0.6196 0.9333 1] Entrance Beacon Setup
        (bind _asbp_dungeon_locs_marker (Utilities|Casting|CastToBP_DungeonLOCs_Marker (Variables|/Script/Engine.ChildActorComponent|GetChildActor (Variables|Default|GetBP_DungeonLOC_Marker))))
        (Class|BeaconManager|RegisterTransientDungeonEntrance _returnvalue_7 _returnvalue _yaw (Transformation|GetWorldLocation (Variables|/Game/Gameplay/Dungeons/BluePrints/BP_DungeonLOCs_Marker.BP_DungeonLOCs_Marker_C|GetBeaconLocation _asbp_dungeon_locs_marker)) _returnvalue_5)
        (Development|PrintText (Utilities|Text|FormatText "Dungeon Registered: {DungeonName}{LF}   Position: {Position}{LF}   Rotation:{Rotation}{LF}   Entrance Index:{EntranceIndex} " _returnvalue_7 (Utilities|Text|MakeLiteralText " 
") (Utilities|String|ToString(Vector) _returnvalue) _yaw _returnvalue_5) false)))))

(event Custom|UpdateInteractCheck
  (bind _interactactor (Variables|Runtime|GetInteractActor))
  (bind _cognitionstimulisource (Variables|/Game/Gameplay/Dungeons/BluePrints/BP_DungeonInteract.BP_DungeonInteract_C|GetCognitionStimuliSource _interactactor))
  ;[1 1 1] Lock, Stat, Mission checks
  (switch Utilities|FlowControl|Switch|SwitchonE_DungeonEntranceLockTypes (Variables|Runtime|GetLockType)
    (:NewEnumerator5
      ;[1 1 1] Register for interact or not based on stat,lock,or mission check
      (Variables|Runtime|SetEnableAudio true :!label _label)
      (Class|AIPerceptionStimuliSourceComponent|RegisterforSense _cognitionstimulisource "/Script/Phoenix.AISense_CogGroup_Interact")
      (CallFunction|AudioCheck))
    (:NewEnumerator0
      (bind _missioncheckpassed (CallFunction|MissionStateCheck))
      (if _missioncheckpassed
        (goto _label)
        (else
          (Variables|Runtime|SetEnableAudio false :!label _label_2)
          (Class|AIPerceptionStimuliSourceComponent|UnregisterfromSense _cognitionstimulisource "/Script/Phoenix.AISense_CogGroup_Interact"))))
    (:NewEnumerator1
      (bind _load (CallFunction|StatCheck))
      (if _load
        (goto _label)
        (else
          (goto _label_2))))
    (:NewEnumerator2
      (bind _lockpassed (CallFunction|LockCheck))
      (if _lockpassed
        (goto _label)
        (else
          (goto _label_2))))
    (:NewEnumerator3
      (bind _checkpassed (CallFunction|DayNightCheck))
      (if _checkpassed
        (goto _label)
        (else
          (goto _label_2))))
    (:NewEnumerator4
      (if (Variables|Runtime|GetSwitchActive)
        (goto _label)
        (else
          (goto _label_2))))))

(event EventSwitchon
  (params (SwitchActor :type Actor%20Object%20Reference))
  (bind _asbp_trigger_volume (Utilities|Casting|CastToBP_TriggerVolume SwitchActor)
    (:then
      (Variables|/Game/Gameplay/Blueprints/Universal/BP_TriggerVolume.BP_TriggerVolume_C|SetInvertToggle _asbp_trigger_volume true)
      (Collision|SetCollisionEnabled (Variables|Default|GetEntranceBlocker) "QueryAndPhysics"))
    (:CastFailed
      _))
  (Variables|Runtime|SetSwitchActive true)
  (CallFunction|UpdateInteractCheck))

(event EventTick
  (params (DeltaSeconds :type Float%20%28single-precision%29))
  ;[1 1 1] Audio
  ;;[1 1 1] Tick: Set RTPC DistanceToPlayer over .3s
  (if (Utilities|IsValid self)
    (Class|AkGameplayStatics|SetRTPCValue 0 (Math|Vector|Distance(Vector) (Transformation|GetActorLocation (Class|BipedPlayer|GettheBipedPlayer)) (Transformation|GetWorldLocation (Variables|Default|GetSphere))) 300 0 "BP_DungeonLOCs_DistanceToPlayer")))

(event EventSwitchOff
  (params (SwitchActor :type Actor%20Object%20Reference))
  (bind _asbp_trigger_volume (Utilities|Casting|CastToBP_TriggerVolume SwitchActor)
    (:then
      (Variables|/Game/Gameplay/Blueprints/Universal/BP_TriggerVolume.BP_TriggerVolume_C|SetInvertToggle _asbp_trigger_volume false)
      (Collision|SetCollisionEnabled (Variables|Default|GetEntranceBlocker) "NoCollision"))
    (:CastFailed
      _))
  (Variables|Runtime|SetSwitchActive false)
  (CallFunction|UpdateInteractCheck))

(event EventBeginPlay
  (bind _dungeonname (Variables|Default|GetDungeonName))
  (Class|HermesBPLibrary|HermesBindEvent (delegate Custom|DungeonLocsInteractUpdate) self)
  (Utilities|FlowControl|Sequence
    (:then_0
      ;[1 1 1] Variable setup
      (bind _asbp_dungeon_interact (Utilities|Casting|CastToBP_DungeonInteract (Variables|/Script/Engine.ChildActorComponent|GetChildActor (Variables|Default|GetInteractChildActor))))
      (Variables|Runtime|SetInteractActor _asbp_dungeon_interact)
      (bind _returnvalue (Utilities|GetDataTableRow (.datatable _dungeonname) (.dungeonname _dungeonname))
        (:then
          (if (Utilities|IsValidSoftObjectReference (Class|PhoenixBPLibrary|CasttoWorldSoftObjectReference (.DungeonLevel (Utilities|Struct|BreakSTR_TransientDungeonListData _returnvalue))))
            (Variables|Runtime|SetWorldToLoad (Class|PhoenixBPLibrary|CasttoWorldSoftObjectReference (.DungeonLevel (Utilities|Struct|BreakSTR_TransientDungeonListData _returnvalue))))))))
    (:then_1
      ;[1 1 1] Audio
      (if (Variables|Runtime|GetEnableAudio)
        (bind _returnvalue_2 (Class|AkGameplayStatics|GetAkComponent 0 "None" (+ (Transformation|GetActorLocation self) "-1230.000000,0.000000,252.000000") "KeepRelativeOffset"))
        (Utilities|IsValid _returnvalue_2
          (:Is%20Valid
            (Class|AkGameObject|PostAkEvent _returnvalue_2 "/Game/WWise/Events/InteractiveObjects/BP_DungeonLOCs/BP_DungeonLOCs_Gate_Energy_Loop.BP_DungeonLOCs_Gate_Energy_Loop")
            (Class|AkComponent|SetStopwhenOwnerDestroyed _returnvalue_2 true)))))
    (:then_2
      (if (.BlockerCollisionOff (Utilities|Struct|BreakSTR_TransientDungeonListData (Variables|Runtime|GetEntranceData)))
        (Collision|SetCollisionEnabled (Variables|Default|GetEntranceBlocker) "NoCollision")))
    (:then_3
      ;[1 1 1] UI said should be at same location as interact.
      (Transformation|SetRelativeLocationAndRotation (Variables|Default|GetBP_DungeonLOC_Marker) "0, 0, 0" "0, 0, 0" false false))))

(event EventExecuteLevelLoad
  (bind _worldtoload (Variables|Runtime|GetWorldToLoad))
  ;[0.9908 1 0.2958] Load Level
  ;;[1 1 1] Resolve ambiguity during automation. Always returns false under normal circumstances
  (bind _returnvalue (Class|MissionManager|AutomationBlocksDungeonLoad (.dungeonname (Variables|Default|GetDungeonName))))
  (if (not _returnvalue)
    (if (.DisableCompanionsOnEnter (Utilities|Struct|BreakSTR_TransientDungeonListData (Variables|Runtime|GetEntranceData)))
      (Class|CompanionManager|DisableSystemicCompanionsforDungeons true))
    (Utilities|FlowControl|Delay 1.0)
    (if (not (.IsExit (Utilities|Struct|BreakSTR_TransientDungeonListData (Variables|Runtime|GetEntranceData))))
      (Class|PhoenixGameInstance|PhoenixOpenLevelbySoftObjectPtr _worldtoload false)
      (else
        ;;[1 1 1] For Exit
        (Class|PhoenixGameInstance|PhoenixOpenLevelbySoftObjectPtr _worldtoload false (Utilities|String|Append (Variables|Runtime|GetPlayerStartTag) (Utilities|String|ToString(Name) (.dungeonname (Variables|Default|GetDungeonName))) "_EXIT"))))
    ;;[1 1 1] For Jim Henn's player transition to new level
    (bind _asphoenix_game_instance (Utilities|Casting|CastToPhoenixGameInstance (Game|GetGameInstance)))
    (Variables|/Script/Phoenix.PhoenixGameInstance|SetRespawnReason _asphoenix_game_instance "TraveledToDungeon")))

(fn ConstructionScript
  (bind _dungeonname (Variables|Default|GetDungeonName))
  (bind _bp_dungeonloc_marker (Variables|Default|GetBP_DungeonLOC_Marker))
  (bind _sanctumtransform (Variables|Default|GetSanctumTransform))
  (bind _parent (Variables|Default|GetParent))
  (Utilities|FlowControl|Sequence
    (:then_0
      ;[1 1 1] Set text for beacons
      (bind _returnvalue (Utilities|GetDataTableRow (.datatable _dungeonname) (.dungeonname _dungeonname))
        (:then
          (bind _output_get (Variables|Runtime|SetEntranceData _returnvalue))
          (if (not (.IsExit (Utilities|Struct|BreakSTR_TransientDungeonListData _output_get)))
            (Variables|Runtime|SetBeaconText (Utilities|String|ToString(Text) (Utilities|Text|ToText(Name) (.dungeonname (Variables|Default|GetDungeonName)))))
            (else
              (Variables|Runtime|SetBeaconText (Utilities|String|Append (Utilities|String|ToString(Name) (.dungeonname (Variables|Default|GetDungeonName))) "_EXIT")))))))
    (:then_1
      ;[1 1 1] Option To Turn OFF GEO for Lightsaber and Text
      (if (.TurnOffMarker (Utilities|Struct|BreakSTR_TransientDungeonListData (Variables|Runtime|GetEntranceData)))
        (Development|SetHiddeninGame _bp_dungeonloc_marker false false)
        (Rendering|SetVisibility _bp_dungeonloc_marker false false)))
    (:then_2
      ;[1 1 1] SetLockState
      (CallFunction|SetLockState))
    (:then_3
      (if (not (.TurnOffGeo (Utilities|Struct|BreakSTR_TransientDungeonListData (Variables|Runtime|GetEntranceData))))
        ;[0.3057 1 0.2258] New Setup Method
        ;;[1 1 1] Look up the model in the DyngeonTypeToMesh, and add it as a child actor component
        (bind _loadedclass (Class|BlueprintHelper|LoadSyncronousActorClass (.Value (Utilities|Map|Find (Variables|Default|GetDungeonTypeToMesh) (.DungeonType (Utilities|Struct|BreakSTR_TransientDungeonListData (Variables|Runtime|GetEntranceData)))))))
        (bind _returnvalue_2 (AddComponent|AddChildActorComponent false))
        (ChildActorComponent|SetChildActorClass (Variables|Default|GetParent) _loadedclass)
        (Transformation|SetWorldTransform _returnvalue_2 (Transformation|GetWorldTransform (Utilities|Select :Index (.DungeonType (Utilities|Struct|BreakSTR_TransientDungeonListData (Variables|Runtime|GetEntranceData))) :NewEnumerator4 _parent :NewEnumerator0 _parent :NewEnumerator10 _parent :NewEnumerator1 (Variables|Default|GetCairnATransform) :NewEnumerator11 _parent :NewEnumerator12 _parent :NewEnumerator2 _parent :NewEnumerator5 _parent :NewEnumerator7 _parent :NewEnumerator6 _parent :NewEnumerator3 _sanctumtransform :NewEnumerator8 _sanctumtransform :NewEnumerator9 _sanctumtransform :NewEnumerator13 (Variables|Default|GetSwimmingTransform) :NewEnumerator14 _parent)) false false)))
    (:then_4
      (Transformation|SetRelativeLocationAndRotation (Variables|Default|GetBP_DungeonLOC_Marker) "0, 0, 0" "0, 0, 0" false false))))

(fn StatCheck
  (bind _entrancedata (Variables|Runtime|GetEntranceData))
  (bind (_statname _neededstatvalue) (Utilities|Struct|BreakSTR_TransientDungeonListData _entrancedata))
  (bind _returnvalue (Class|StatsManager|GetStatName _statname))
  (if (Utilities|Name|NotEqual(Name) _returnvalue "None")
    (bind _returnvalue_2 (Class|StatsManager|ReadStat _returnvalue)))
  (return (== _returnvalue_2 _neededstatvalue)))

(fn LockCheck
  (bind _entrancedata (Variables|Runtime|GetEntranceData))
  (bind (_lockid _neededlockstate) (Utilities|Struct|BreakSTR_TransientDungeonListData _entrancedata))
  (bind _returnvalue (Class|LockManagerInterface|GetState _lockid))
  (return (Utilities|Enum|Equal(Enum) _returnvalue _neededlockstate)))

(fn MissionStateCheck
  (bind _entrancedata (Variables|Runtime|GetEntranceData))
  (bind (_missionlock _missionstaterequired) (Utilities|Struct|BreakSTR_TransientDungeonListData _entrancedata))
  (bind _name (Utilities|Struct|BreakDatabaseMissionList _missionlock))
  (if (Utilities|Name|NotEqual(Name) _name "None")
    (bind _returnvalue (Class|MissionManager|GetMissionStatusBP _name))
    (if (or (Utilities|Enum|Equal(Enum) _returnvalue _missionstaterequired) (Utilities|Enum|Equal(Enum) _returnvalue "MISSION_STATUS_COMPLETE"))
      (LocalVariables|SetPassed (or (Utilities|Enum|Equal(Enum) _returnvalue _missionstaterequired) (Utilities|Enum|Equal(Enum) _returnvalue "MISSION_STATUS_COMPLETE")))
      (return (LocalVariables|GetPassed)))
    (else
      (LocalVariables|SetPassed false)
      (return (LocalVariables|GetPassed)))))

(fn SetLockState
  (bind _entrancedata (Variables|Runtime|GetEntranceData))
  (bind (_missionlock _usemissioncheck _usestatcheck _uselockcheck _requireswitch _usetimeofdaycheck) (Utilities|Struct|BreakSTR_TransientDungeonListData _entrancedata))
  (if _usemissioncheck
    (Variables|Runtime|SetLockType "NewEnumerator0")
    (elif _usestatcheck
      (Variables|Runtime|SetLockType "NewEnumerator1")
      (elif _uselockcheck
        (Variables|Runtime|SetLockType "NewEnumerator2")
        (elif _requireswitch
          (Variables|Runtime|SetLockType "NewEnumerator4")
          (elif _usetimeofdaycheck
            (Variables|Runtime|SetLockType "NewEnumerator3")
            (else
              (Variables|Runtime|SetLockType "NewEnumerator5"))))))))

(fn DayNightCheck
  ;[1 1 1] Only Work After FGM_01
  (bind _returnvalue (Class|MissionManager|GetMissionStatusBP "FGM_01"))
  (switch Utilities|FlowControl|Switch|SwitchonMissionStatus _returnvalue
    (:MISSION_STATUS_COMPLETE
      (bind _returnvalue_2 (Class|Scheduler|Get))
      (if (Class|Scheduler|IsNight _returnvalue_2)
        (LocalVariables|SetLocalCheck true)
        (else
          (LocalVariables|SetLocalCheck false)))
      (return (LocalVariables|GetLocalCheck)))))

(fn GetDungeonTypefromName
  (params (DungeonTypeName :type Name))
  (switch name DungeonTypeName
    (:Default
      (return "NewEnumerator4"))
    (:Castle%20A
      (return "NewEnumerator0"))
    (:Castle%20B
      (return "NewEnumerator10"))
    (:Cairn%20A
      (return "NewEnumerator1"))
    (:Cairn%20B
      (return "NewEnumerator11"))
    (:Cairn%20C
      (return "NewEnumerator12"))
    (:Cavern
      (return "NewEnumerator2"))
    (:Cavern%20Spider
      (return "NewEnumerator5"))
    (:Cavern%20Dragon
      (return "NewEnumerator7"))
    (:Cavern%20Goblin
      (return "NewEnumerator6"))
    (:Pensieve
      (return "NewEnumerator3"))
    (:Merlin%20Trials
      (return "NewEnumerator8"))
    (:Special
      (return "NewEnumerator9"))
    (:Swimming
      (return "NewEnumerator13"))
    (:HM%20Cart
      (return "NewEnumerator14"))))

(fn GetDungeonDatatableHandle
  (bind _dungeonname (Variables|Default|GetDungeonName))
  (return (Utilities|Struct|MakeDataTableRowHandle (.datatable _dungeonname) (.dungeonname _dungeonname))))

(fn GetUniqueBeaconId
  (bind _dungeonname (Variables|Default|GetDungeonName))
  (bind _returnvalue (Utilities|String|ToString(Name) (.dungeonname _dungeonname)))
  (bind _returnvalue_2 (Utilities|String|Replace _returnvalue "Gobmine" "GobMine"))
  (return (Utilities|String|StringToName (Utilities|String|Append (Utilities|String|SelectString (Utilities|String|Append _returnvalue_2 "_EXIT") _returnvalue_2 (.IsExit (Utilities|Struct|BreakSTR_TransientDungeonListData (Variables|Runtime|GetEntranceData)))) (Utilities|String|ToString(Integer) (Variables|Default|GetEntranceIndex))))))