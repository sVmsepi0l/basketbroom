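; Dungeon exit actor that returns the player from a dungeon to the overland.
; It registers a beacon, pulls prompt text from dungeon data tables, and enables interaction on player overlap once active, optionally requiring a switch.
; Interacting warns during exclusive missions, offering abandonment; otherwise it can re-enable systemic companions, sets the respawn reason and opens the target level.
; The player-start tag derives from the current level name, with a suffix for second exits.
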(event OnComponentBeginOverlap(Sphere)
  (params (OverlappedComponent :type Primitive%20Component%20Object%20Reference) (OtherActor :type Actor%20Object%20Reference) (OtherComp :type Primitive%20Component%20Object%20Reference) (OtherBodyIndex :type Integer) (bFromSweep :type Boolean) (SweepResult :type Hit%20Result%20Structure%20%28by%20ref%29))
  (if (not (Variables|Default|GetOneWay))
    (Utilities|FlowControl|Gate (Variables|Default|GetExitPrompt))))

(event OnComponentBeginOverlap(TextSphere)
  (params (OverlappedComponent :type Primitive%20Component%20Object%20Reference) (OtherActor :type Actor%20Object%20Reference) (OtherComp :type Primitive%20Component%20Object%20Reference) (OtherBodyIndex :type Integer) (bFromSweep :type Boolean) (SweepResult :type Hit%20Result%20Structure%20%28by%20ref%29))
  ;[1 1 1] We Cast to biped player, because player mounts also collide with PlayerOnly Collision
  (Utilities|Casting|CastToBiped_Player OtherActor)
  (if (Variables|Default|GetIsActive)
    (Class|AIPerceptionStimuliSourceComponent|RegisterforSense (Variables|Default|GetCognitionStimuliSource) "/Script/Phoenix.AISense_CogGroup_Interact")))

(event OnComponentEndOverlap(TextSphere)
  (params (OverlappedComponent :type Primitive%20Component%20Object%20Reference) (OtherActor :type Actor%20Object%20Reference) (OtherComp :type Primitive%20Component%20Object%20Reference) (OtherBodyIndex :type Integer))
  ;[1 1 1] We Cast to biped player, because player mounts also collide with PlayerOnly Collision
  (Utilities|Casting|CastToBiped_Player OtherActor)
  (if (Variables|Default|GetIsActive)
    (Class|AIPerceptionStimuliSourceComponent|UnregisterfromSense (Variables|Default|GetCognitionStimuliSource) "/Script/Phoenix.AISense_CogGroup_Interact")))

(event Custom|Trigger%20Return%20To%20Overland
  ;[1 1 1] Debug for Easy Triggering - Added by Corey
  (Utilities|AVAMacroLoadtoOverland))

(event Custom|PopupCompleted
  (params (PopupScreen :type Popup%20Screen%20Object%20Reference) (CompletionActionIndex :type Integer))
  ;[1 1 1] Warn if on exclusive mission
  (switch int CompletionActionIndex
    (:0
      (Class|MissionManager|AbandonMissionBP))
    (:1
      (Utilities|FlowControl|Delay 2.0)
      (Class|AIPerceptionStimuliSourceComponent|RegisterforSense (Variables|Default|GetCognitionStimuliSource) "/Script/Phoenix.AISense_CogGroup_Interact"))))

(event Custom|DungeonExitExclusiveUnlock
  (params (Caller :type Object%20Object%20Reference))
  (Variables|Default|SetDoExclusiveCheck false))

(event Custom|ForceLevelChange
  (Class|AIPerceptionStimuliSourceComponent|UnregisterfromSense (Variables|Default|GetCognitionStimuliSource) "/Script/Phoenix.AISense_CogGroup_Interact")
  (if (Variables|Default|GetDoExclusiveCheck)
    (bind _returnvalue (Class|MissionBPLibrary|IsExclusiveMissionActive))
    (if _returnvalue
      ;[1 1 1] Warn if on exclusive mission
      (bind _returnvalue_2 (Class|UIManager|Get))
      (bind _returnvalue_3 (Class|UIManager|ShowYesNoPopup _returnvalue_2 (Variables|Default|GetFailWarningTitleString) (Variables|Default|GetFailWarningDescriptionString) false true 0 "UIPP_Important" true))
      (EventDispatchers|BindEventtoPopupButtonPressCompletedEvent _returnvalue_3 (delegate Custom|PopupCompleted))
      (else
        ;[1 1 1] Turn systemic companions back on for DADA dungeons.
        (if (Variables|Default|GetEnableSystemicCompanion) :!label _label
          (Class|CompanionManager|DisableSystemicCompanionsforDungeons false))
        ;[1 1 1] For Jim Henn's player transition to new level
        (bind _asphoenix_game_instance (Utilities|Casting|CastToPhoenixGameInstance (Game|GetGameInstance))
          (:then
            (Variables|/Script/Phoenix.PhoenixGameInstance|SetRespawnReason _asphoenix_game_instance "TraveledFromDungeon"))
          (:CastFailed
            _))
        (Utilities|AVAMacroLoadtoOverland)))
    (else
      (goto _label))))

(event EventBeginPlay
  (Class|HermesBPLibrary|HermesBindEvent (delegate Custom|DungeonExitExclusiveUnlock))
  ;[1 1 1] Register for use with beacons
  (bind _returnvalue (CallFunction|GetUniqueBeaconId))
  (Class|BeaconManager|RegisterDungeonExit (Transformation|GetActorLocation) _returnvalue false)
  ;[1 1 1] Get exit text from data table
  (CallFunction|UpdateInteractText)
  (if (Variables|Default|GetRequireSwitch)
    (Class|AIPerceptionStimuliSourceComponent|UnregisterfromSense (Variables|Default|GetCognitionStimuliSource) "/Script/Phoenix.AISense_CogGroup_Interact")
    (else
      (Variables|Default|SetIsActive true)))
  ;[1 1 1] Audio
  (if (Variables|Default|GetIsActive)
    (Class|AkGameObject|PostAkEvent (Variables|Default|GetAk_BP_WorldTeleport) "/Game/WWise/Events/InteractiveObjects/BP_WorldTeleport/BP_WorldTeleport_Gate_Energy_Loop.BP_WorldTeleport_Gate_Energy_Loop") ; SFX
  ))

(event EventInteract
  (params (AvaService :type BT%20Service%20Ava%20AI%20Tree%20Object%20Reference))
  (Class|AIPerceptionStimuliSourceComponent|UnregisterfromSense (Variables|Default|GetCognitionStimuliSource) "/Script/Phoenix.AISense_CogGroup_Interact")
  (if (Variables|Default|GetDoExclusiveCheck)
    (bind _returnvalue (Class|MissionBPLibrary|IsExclusiveMissionActive))
    (if _returnvalue
      ;[1 1 1] Warn if on exclusive mission
      (bind _returnvalue_2 (Class|UIManager|Get))
      (bind _returnvalue_3 (Class|UIManager|ShowYesNoPopup _returnvalue_2 (Variables|Default|GetFailWarningTitleString) (Variables|Default|GetFailWarningDescriptionString) false true 0 "UIPP_Important" true))
      (EventDispatchers|BindEventtoPopupButtonPressCompletedEvent _returnvalue_3 (delegate Custom|PopupCompleted))
      (else
        ;[1 1 1] Turn systemic companions back on for DADA dungeons.
        (if (Variables|Default|GetEnableSystemicCompanion) :!label _label
          (Class|CompanionManager|DisableSystemicCompanionsforDungeons false))
        ;[1 1 1] For Jim Henn's player transition to new level
        (bind _asphoenix_game_instance (Utilities|Casting|CastToPhoenixGameInstance (Game|GetGameInstance))
          (:then
            (Variables|/Script/Phoenix.PhoenixGameInstance|SetRespawnReason _asphoenix_game_instance "TraveledFromDungeon"))
          (:CastFailed
            _))
        (Utilities|AVAMacroLoadtoOverland)))
    (else
      (goto _label))))

(event EventSwitchon
  (params (SwitchActor :type Actor%20Object%20Reference))
  (Variables|Default|SetIsActive true))

(event EventOnRestorefromSave
  (params (AutosaveActor :type BP%20Autosave%20Trigger%20Object%20Reference))
  (Variables|Default|SetIsActive true))

(fn ConstructionScript
  (bind _returnvalue (Game|GetCurrentLevelName true))
  (bind _output_get (Variables|Default|SetLevelName _returnvalue))
  (Rendering|Components|TextRender|SetText (Variables|Default|GetTextRender) (Utilities|Text|ToText(String) (Utilities|String|Append "Current Level " _output_get)))
  (bind _returnvalue_2 (Utilities|GetDataTableRow (Variables|Default|GetDungeonTable) (Utilities|String|StringToName (Variables|Default|GetLevelName)))
    (:then
      (Variables|Default|SetLoadingToLevel (select (Variables|Default|GetThis%20is%20a%20second%20_EXIT) (.DungeonSecondExitLoadingString (Utilities|Struct|BreakSTR_DungeonListData _returnvalue_2)) (.DungeonExitLoadingString (Utilities|Struct|BreakSTR_DungeonListData _returnvalue_2)))))
    (:RowNotFound
      (bind _returnvalue_3 (Class|ModGameSupport|GetCompositeDataTablefromBase "/Game/Data/Dungeons/DT_TransientDungeonsTable.DT_TransientDungeonsTable"))
      (bind _returnvalue_4 (Utilities|GetDataTableRow _returnvalue_3 (Utilities|String|StringToName (Variables|Default|GetLevelName)))
        (:then
          (Variables|Default|SetLoadingToLevel (select (Variables|Default|GetThis%20is%20a%20second%20_EXIT) (.DungeonSecondExitLoadingString (Utilities|Struct|BreakSTR_TransientDungeonListData _returnvalue_4)) (.DungeonExitLoadingString (Utilities|Struct|BreakSTR_TransientDungeonListData _returnvalue_4)))))))))

(fn UpdateInteractText
  (bind _returnvalue (Game|GetCurrentLevelName true))
  (bind _returnvalue_2 (Utilities|GetDataTableRow (Variables|Default|GetDungeonTable) (Utilities|String|StringToName _returnvalue))
    (:then
      (Variables|Default|SetLoadingToLevel (select (Variables|Default|GetThis%20is%20a%20second%20_EXIT) (.DungeonSecondExitLoadingString (Utilities|Struct|BreakSTR_DungeonListData _returnvalue_2)) (.DungeonExitLoadingString (Utilities|Struct|BreakSTR_DungeonListData _returnvalue_2)))))
    (:RowNotFound
      (bind _returnvalue_3 (Class|ModGameSupport|GetCompositeDataTablefromBase "/Game/Data/Dungeons/DT_TransientDungeonsTable.DT_TransientDungeonsTable"))
      (bind _returnvalue_4 (Utilities|GetDataTableRow _returnvalue_3 (Utilities|String|StringToName _returnvalue))
        (:then
          (Variables|Default|SetLoadingToLevel (select (Variables|Default|GetThis%20is%20a%20second%20_EXIT) (.DungeonSecondExitLoadingString (Utilities|Struct|BreakSTR_TransientDungeonListData _returnvalue_4)) (.DungeonExitLoadingString (Utilities|Struct|BreakSTR_TransientDungeonListData _returnvalue_4))))))))
  (Variables|/Script/Cognition.CognitionStimuliSourceComponent|SetTargetText (Variables|Default|GetCognitionStimuliSource) (Variables|Default|GetLoadingToLevel)))

(fn GetUniqueBeaconId
  (if (Utilities|Name|Equal(Name) (Variables|Default|GetBeaconID) "None")
    (return (Utilities|String|StringToName (Utilities|GetObjectName self)))
    (else
      (return (Variables|Default|GetBeaconID)))))